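; Teleport projectile that moves the player to its impact point when it hits a flat, upward-facing surface.
; On spawn it disables firing, then re-enables it and destroys itself after a three-second delay if nothing is hit.
; Any mesh hit also restores firing and destroys the projectile, but only a straight-up hit normal, within a small tolerance, triggers the teleport.
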(event `self.ReceiveBeginPlay`
  ;[1 1 1] Activa y desactiva el disparo y destruye el actor luego de n segundos
  (`self.SetCanFire` false)
  (`KismetSystemLibrary.Delay` 3.0)
  (`self.SetCanFire` true)
  (`self.K2_DestroyActor`))

(event `self.ProjectileMesh.OnComponentHit`
  (params (HitComponent :type "PrimitiveComponent Object Reference") (OtherActor :type "Actor Object Reference") (OtherComp :type "PrimitiveComponent Object Reference") (NormalImpulse :type "Vector Structure") (Hit :type "HitResult Structure (by ref)"))
  (bind (_bblockinghit _binitialoverlap _time _distance _location _impactpoint _normal) (`GameplayStatics.BreakHitResult` Hit))
  ;[1 1 1] Teletransporta al player en el primer Hit
  (if (== _normal (0.0 0.0 1.0))
    (`self.TeleportPlayer` _location))
  (`self.SetCanFire` true)
  (`self.K2_DestroyActor`))

(fn `UserConstructionScript`
  (`parent.UserConstructionScript`))