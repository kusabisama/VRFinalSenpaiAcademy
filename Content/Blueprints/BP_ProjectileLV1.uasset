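; BP_ProjectileLV1 is a teleport projectile that moves the player character to where it lands on a flat, upward-facing surface.
; On a mesh hit it compares the hit normal to world up with a tight tolerance, so slopes, walls and ceilings do not trigger a teleport.
; A match calls TeleportPlayer, which sets player 0's location without sweep, then prints the location.
; The projectile destroys itself on any hit.
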(event `self.ProjectileMesh.OnComponentHit`
  (params (HitComponent :type "PrimitiveComponent Object Reference") (OtherActor :type "Actor Object Reference") (OtherComp :type "PrimitiveComponent Object Reference") (NormalImpulse :type "Vector Structure") (Hit :type "HitResult Structure (by ref)"))
  (bind (_bblockinghit _binitialoverlap _time _distance _location _impactpoint _normal) (`GameplayStatics.BreakHitResult` Hit))
  ;[0 0 0] Teletransporta al player en el primer Hit
  (if (== _normal (0.0 0.0 1.0))
    (`self.TeleportPlayer` _location)
    (`KismetSystemLibrary.PrintString` (`KismetStringLibrary.Conv_VectorToString` _location))
    (`self.K2_DestroyActor`)
    (else
      (`self.K2_DestroyActor`))))

(fn `TeleportPlayer`
  (params (TeleportLocation :type "Vector Structure"))
  (`self.K2_SetActorLocation` (`GameplayStatics.GetPlayerCharacter` 0) TeleportLocation false true))

(fn `UserConstructionScript`)