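; Platform Blueprint that calls ActivatePlataform, defined outside this graph, in response to switch events, likely to show or hide itself.
; The construction script runs the parent's and calls the same function when Hide is set.
; The Switch event also prints a debug "Hello".
; A dispatcher version binding Delegate to each referenced ring switch is left disconnected, and BeginPlay is empty.
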(event `self.ReceiveBeginPlay`)

(event `Delegate`
  ;[0.2292 0.2292 0.2292] Version Dispatchers
  (`self.ActivatePlataform`))

(event `/Game/Blueprints/Interfaces/I_Switchable.Switch`
  (`self.ActivatePlataform`)
  (`KismetSystemLibrary.PrintString` "Hello"))

(fn `UserConstructionScript`
  (`parent.UserConstructionScript`)
  (if (`self.Hide`)
    (`self.ActivatePlataform`)))