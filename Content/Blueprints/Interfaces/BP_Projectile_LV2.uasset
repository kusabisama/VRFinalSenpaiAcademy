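; Level 2 projectile Blueprint that teleports the player to where it lands on upward-facing surfaces.
; On spawn it changes the can-fire state, then resets it and destroys itself after a short lifetime.
; A mesh hit also resets that state and destroys the projectile, first teleporting the player to the hit location only if the surface normal is close to vertical.
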(event `self.ReceiveBeginPlay`
  ;[1 1 1] Activa y desactiva el disparo y destruye el actor luego de n segundos
  (`self.SetCanFire` "NewEnumerator3")
  (`KismetSystemLibrary.Delay` 2.0)
  (`self.SetCanFire` "NewEnumerator0")
  (`self.K2_DestroyActor`))

(event `self.ProjectileMesh.OnComponentHit`
  (params (HitComponent :type "PrimitiveComponent Object Reference") (OtherActor :type "Actor Object Reference") (OtherComp :type "PrimitiveComponent Object Reference") (NormalImpulse :type "Vector Structure") (Hit :type "HitResult Structure (by ref)"))
  (bind (_bblockinghit _binitialoverlap _time _distance _location _impactpoint _normal) (`GameplayStatics.BreakHitResult` Hit))
  (if (>= (.z _normal) 0.8)
    (`self.TeleportPlayer` _location)
    (`self.SetCanFire` "NewEnumerator0")
    (`self.K2_DestroyActor`)
    (else
      (`self.SetCanFire` "NewEnumerator0")
      (`self.K2_DestroyActor`))))

(fn `UserConstructionScript`
  (`parent.UserConstructionScript`))