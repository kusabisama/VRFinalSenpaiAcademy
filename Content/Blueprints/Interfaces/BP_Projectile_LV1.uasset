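; Level 1 projectile that teleports the player to where it lands, provided the surface faces mostly upward.
; On spawn it changes the can-fire state, then restores it and destroys itself after a short lifetime.
; The first mesh hit checks the normal's Z before teleporting and drawing a debug point.
; Any hit, valid or not, resets the fire state and destroys the projectile.
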(event `self.ReceiveBeginPlay`
  ;[1 1 1] Activa y desactiva el disparo y destruye el actor luego de n segundos
  (`self.SetCanFire` "NewEnumerator3")
  (`KismetSystemLibrary.Delay` 2.0)
  (`self.SetCanFire` "NewEnumerator0")
  (`self.K2_DestroyActor`))

(event `self.ProjectileMesh.OnComponentHit`
  (params (HitComponent :type "PrimitiveComponent Object Reference") (OtherActor :type "Actor Object Reference") (OtherComp :type "PrimitiveComponent Object Reference") (NormalImpulse :type "Vector Structure") (Hit :type "HitResult Structure (by ref)"))
  (bind (_bblockinghit _binitialoverlap _time _distance _location _impactpoint _normal) (`GameplayStatics.BreakHitResult` Hit))
  ;[1 1 1] Teletransporta al player en el primer Hit
  (if (>= (.z _normal) 0.8)
    (`self.TeleportPlayer` _impactpoint)
    (`KismetSystemLibrary.DrawDebugPoint` _impactpoint 30.0 (struct :`R` 0.223093 :`G` 1.0 :`A` 1.0) 10.0))
  (`self.SetCanFire` "NewEnumerator0")
  (`self.K2_DestroyActor`))

(fn `UserConstructionScript`
  (`parent.UserConstructionScript`))