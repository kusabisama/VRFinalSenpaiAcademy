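; Level 3 projectile that toggles the player's teleport fire action according to the ground beneath it.
; After a brief startup cooldown, each Tick traces downward and treats a sufficiently upward-facing hit normal as valid ground.
; The result sets TypeActionFire on the FirstPersonCharacter and prints a colored OK/NO debug message.
; BeginPlay changes the can-fire state, then restores it and destroys the projectile after a fixed delay.
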(event `self.ReceiveTick`
  (params (DeltaSeconds :type "Float (single-precision)"))
  (bind (_returnvalue_x _returnvalue_y _returnvalue_z) (`KismetMathLibrary.BreakVector` (`self.K2_GetActorLocation`)))
  (bind _outhit (`KismetSystemLibrary.LineTraceSingleForObjects` (`KismetMathLibrary.MakeVector` _returnvalue_x _returnvalue_y _returnvalue_z) (`KismetMathLibrary.MakeVector` _returnvalue_x _returnvalue_y (+ _returnvalue_z -1000.0)) (`|MakeArray` "ObjectTypeQuery1" :!type "EObjectTypeQuery Enum")))
  (set `self.NormalImpactPoint` (`.Normal` (`GameplayStatics.BreakHitResult` _outhit)))
  (if (`self.InitialTeleportCooldown`)
    (`self.SetTypeActionFire`)))

(event `self.ReceiveBeginPlay`
  (`|ExecutionSequence`
    (:`then_0`
      ;[1 1 1] Activa y desactiva el disparo y destruye el actor luego de n segundos
      (`self.SetCanFire` "NewEnumerator3")
      (`KismetSystemLibrary.Delay` 3.0)
      (`/Engine/EditorBlueprintResources/StandardMacros.IsValid` self
        (:`Is Valid`
          (`self.SetCanFire` "NewEnumerator0")
          (`self.K2_DestroyActor`))))
    (:`then_1`
      (set `self.InitialTeleportCooldown` false)
      (`KismetSystemLibrary.Delay` 0.1)
      (set `self.InitialTeleportCooldown` true))))

(event `SetTypeActionFire`
  (bind (_normalimpactpoint_x _normalimpactpoint_y _normalimpactpoint_z) (`KismetMathLibrary.BreakVector` (`self.NormalImpactPoint`)))
  ;[1 1 1] Controla si hay suelo debajo y activa o desactiva la teletrasportacion
  (if (>= _normalimpactpoint_z 0.8)
    (bind _asfirst_person_character (cast `/Game/Blueprints/FirstPersonCharacter` (`GameplayStatics.GetPlayerCharacter` 0)))
    (set `/Game/Blueprints/FirstPersonCharacter.TypeActionFire` "NewEnumerator2" _asfirst_person_character)
    (`KismetSystemLibrary.PrintString` "OK" true true (struct :`G` 1.0 :`B` 0.209817 :`A` 1.0) 0.3)
    (else
      (bind _asfirst_person_character_2 (cast `/Game/Blueprints/FirstPersonCharacter` (`GameplayStatics.GetPlayerCharacter` 0)))
      (set `/Game/Blueprints/FirstPersonCharacter.TypeActionFire` "NewEnumerator3" _asfirst_person_character_2)
      (`KismetSystemLibrary.PrintString` "NO" true true (struct :`R` 1.0 :`G` 0.100414 :`B` 0.050654 :`A` 1.0) 0.3))))

(fn `UserConstructionScript`
  (`parent.UserConstructionScript`))