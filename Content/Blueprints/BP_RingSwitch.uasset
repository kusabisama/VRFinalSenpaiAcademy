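; Ring switch that messages a list of linked hide-switch platforms when a projectile overlaps it.
; Tick spins the ring mesh on pitch by RotationSpeed per frame, without delta-time scaling.
; ProjectileOverlap validates only the first list entry, then calls SwitchMessage on every platform and prints its name for debugging.
; An event dispatcher alternative is left unconnected, and a note reports the overlap firing twice.
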(event `self.ReceiveTick`
  (params (DeltaSeconds :type "Float (single-precision)"))
  (if (> (`self.RotationSpeed`) 0.0)
    (`SceneComponent.K2_AddLocalRotation` (`self.RingMesh`) (`KismetMathLibrary.MakeRotator` 0.0 (`self.RotationSpeed`)) false false)))

(event `self.ProjectileOverlap`
  (params (ProjectilRef :type "/Game/Base/BP_Projectile Object Reference"))
  (bind _plataformhideswitchlist (`self.PlataformHideSwitchList`))
  ;[1 0 0] Esta iniciando dos veces
  (`/Engine/EditorBlueprintResources/StandardMacros.IsValid` (`|GetArrayItem` _plataformhideswitchlist)
    (:`Is Valid`
      (for _array_element _plataformhideswitchlist
        (message `/Game/Blueprints/Interfaces/I_Switchable.Switch` _array_element)
        (`KismetSystemLibrary.PrintString` (`KismetSystemLibrary.GetDisplayName` _array_element) true true (struct :`G` 1.0 :`B` 0.58936 :`A` 1.0))))))

(fn `UserConstructionScript`
  (`parent.UserConstructionScript`))