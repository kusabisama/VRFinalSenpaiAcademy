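; BP_Platform is a base platform actor that can be switched between present and absent.
; ActivatePlataform toggles visibility from the root down and uses a FlipFlop to alternate CollisionMesh collision, disabling it on the first call.
; The construction script turns off collision on the render mesh, leaving it to the separate CollisionMesh.
; When a FirstPersonCharacter overlaps PlatformArea it calls DetectChar, which is empty here.
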(event `ActivatePlataform`
  (bind _collisionmesh (`self.CollisionMesh`))
  ;[1 1 1] Armado y Desarmado de plataforma
  (`SceneComponent.ToggleVisibility` (`self.Root`) true)
  (`/Engine/EditorBlueprintResources/StandardMacros.FlipFlop`
    (:`A`
      (`PrimitiveComponent.SetCollisionEnabled` _collisionmesh "NoCollision"))
    (:`B`
      (`PrimitiveComponent.SetCollisionEnabled` _collisionmesh "QueryAndPhysics"))))

(event `self.PlatformArea.OnComponentBeginOverlap`
  (params (OverlappedComponent :type "PrimitiveComponent Object Reference") (OtherActor :type "Actor Object Reference") (OtherComp :type "PrimitiveComponent Object Reference") (OtherBodyIndex :type Integer) (bFromSweep :type Boolean) (SweepResult :type "HitResult Structure (by ref)"))
  (cast `/Game/Blueprints/FirstPersonCharacter` OtherActor)
  (`self.DetectChar`))

(fn `DetectChar`)

(fn `UserConstructionScript`
  (`PrimitiveComponent.SetCollisionEnabled` (`self.PlatformMesh`) "NoCollision") ; Desactivo la Collision de la Mesh de Render
)