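; Base projectile Blueprint that provides movement setup and player-interaction helpers for projectiles fired in a first-person game.
; The construction script applies and prints its InitialSpeed, then BeginPlay overwrites the movement component's initial speed with the FirstPersonCharacter's ProjectileImpulse.
; TeleportPlayer moves player 0 to slightly above a given location without sweeping.
; SetCanFire passes an action-fire type to the character to enable or disable firing another projectile.
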(event `self.ReceiveBeginPlay`
  (bind _asfirst_person_character (cast `/Game/Blueprints/FirstPersonCharacter` (`GameplayStatics.GetPlayerCharacter` 0)))
  (set `ProjectileMovementComponent.InitialSpeed` (`/Game/Blueprints/FirstPersonCharacter.ProjectileImpulse` _asfirst_person_character) (`self.ProjectileMovement`)))

(fn `SetCanFire`
  (params (TypeActionFire :type "/Game/Base/Enum_TypeActionFire Enum" :default "NewEnumerator0"))
  ;[1 1 1] Activa o desactiva el disparo de otro Projectil en el FirstPersonCharacer
  (bind _asfirst_person_character (cast `/Game/Blueprints/FirstPersonCharacter` (`GameplayStatics.GetPlayerCharacter` 0)))
  (message `/Game/Blueprints/Interfaces/I_TpOnHItProjectile.SetTypeActionFire` _asfirst_person_character TypeActionFire))

(fn `TeleportPlayer`
  (params (TeleportLocation :type "Vector Structure"))
  (`self.K2_SetActorLocation` (`GameplayStatics.GetPlayerCharacter` 0) (`KismetMathLibrary.MakeVector` TeleportLocation_X TeleportLocation_Y (+ TeleportLocation_Z 30.0)) false true))

(fn `UserConstructionScript`
  (bind _output_get (set `ProjectileMovementComponent.InitialSpeed` (`self.InitialSpeed`) (`self.ProjectileMovement`)))
  (`KismetSystemLibrary.PrintString` (`KismetStringLibrary.Conv_DoubleToString` _output_get)))