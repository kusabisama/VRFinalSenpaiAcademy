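; Base actor for interactable objects that can be selected, deselected and activated.
; Select and deselect events toggle a Selected flag and call matching Select and Deselect functions; while selected, Tick spins the mesh on all three axes at a Speed-scaled rate.
; Activation calls ActivateInteractable and plays a plastic button sound at the actor's location.
; All three called functions are empty here, apparently serving as hooks for child Blueprints.
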(event `self.ReceiveTick`
  (params (DeltaSeconds :type "Float (single-precision)"))
  (bind _returnvalue (* DeltaSeconds (`self.Speed`)))
  (if (`self.Selected`)
    (`SceneComponent.K2_AddLocalRotation` (`self.MeshInteractable`) (`KismetMathLibrary.MakeRotator` _returnvalue _returnvalue _returnvalue) false false)))

(event `/Game/Blueprints/Interfaces/I_Interactable.SelectInteract`
  (set `self.Selected` true)
  (`self.Select`))

(event `/Game/Blueprints/Interfaces/I_Interactable.DeselectInteract`
  (set `self.Selected` false)
  (`self.Deselect`))

(event `/Game/Blueprints/Interfaces/I_Interactable.Activate`
  (`self.ActivateInteractable`)
  (`GameplayStatics.PlaySoundAtLocation` "/Game/Sounds/buttonPlastic.buttonPlastic" (`self.K2_GetActorLocation`) (struct) 1.0 1.0 0.0 null null null))

(fn `ActivateInteractable`)

(fn `Deselect`)

(fn `Select`)

(fn `UserConstructionScript`)